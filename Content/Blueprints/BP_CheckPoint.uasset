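; BP_CheckPoint is a checkpoint actor that records a respawn-style location when the player reaches it.
; When the player pawn overlaps its Box component, it writes its own location into the CP variable on the third-person controller, prints a debug message, and destroys itself, so each checkpoint triggers only once.
; A leftover, unconnected LastCheckPoint assignment never runs.
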(event `CustomEvent`)

(event `self.Box.OnComponentBeginOverlap`
  (params (OverlappedComponent :type "PrimitiveComponent Object Reference") (OtherActor :type "Actor Object Reference") (OtherComp :type "PrimitiveComponent Object Reference") (OtherBodyIndex :type Integer) (bFromSweep :type Boolean) (SweepResult :type "HitResult Structure (by ref)"))
  (if (== OtherActor (`GameplayStatics.GetPlayerPawn` 0))
    (bind _asbp_third_person_player_controller (`/Game/Blueprints/character/BF_FC_communs.GetThirsPersonController`))
    (set `/Game/Blueprints/Main/BP_ThirdPersonPlayerController.CP` (`self.K2_GetActorLocation` self) _asbp_third_person_player_controller)
    (`KismetSystemLibrary.PrintString` "newCP")
    (`self.K2_DestroyActor`)))

(fn `UserConstructionScript`)